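; BP_Pawn_TTBoyB is a modular teen boy pawn that can randomize its outfit.
; The construction script binds the clothing and accessory meshes to the main Mesh as master pose component, then runs the Randomizer.
; When Randomize is set, it rolls glasses, jacket and hood variant once and clears the flag.
; Visibility is reapplied from the stored booleans on every construction, with exactly one of the two hood meshes shown.
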(fn ConstructionScript
  (Class|SkinnedMeshComponent|SetMasterPoseComponent (Variables|Default|GetTTSweater) (Variables|Default|GetMesh) false)
  (|Randomizer))